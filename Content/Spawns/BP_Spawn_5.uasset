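; Wave spawner that releases male and female, walking and running zombies at random reachable navmesh points around itself.
; BeginPlay shows wave-number widgets, then a delayed-loop macro spawns staggered hordes scaled by wave number, with runners joining in later waves.
; Kill delegates empty per-type arrays and set all-dead flags, which Tick polls to start the next wave.
; FunSpawnZombies and SpawnZombie duplicate the inline spawn logic but are never called here.
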(event `self.ReceiveBeginPlay`
  ;[1 1 1] Début du jeu - Spawn par vague
  (`KismetSystemLibrary.Delay` 1.0)
  (set `self.waveNbr` 1)
  (`KismetSystemLibrary.Delay` 1.0)
  ;[1 1 1] Créer le widget pour afficher le num de la vague et appel la fonction spawn zombies
  (`self.createWidgets` :!label _label)
  (`KismetSystemLibrary.Delay` 1.0)
  (bind _foundwidgets (`WidgetBlueprintLibrary.GetAllWidgetsOfClass` "/Game/UI/WaveNumber.WaveNumber_C"))
  (`Widget.RemoveFromParent` _foundwidgets)
  ;[1 1 1] Initialisation & augmente num vague
  (set `self.waveNbr` (+ (`self.waveNbr`) 1))
  (`self.forLoopWithDelay` 0 (* (`self.HordMin`) (`self.waveNbr`)) :!label _label_2
    (:`LoopBody`
      (`|ExecutionSequence`
        (:`then_0`
          (`|ExecutionSequence`
            (:`then_0`
              ;[1 1 1] Fait spawner les zombies male walking
              (if (> (`self.waveNbr`) 1)
                (bind _returnvalue (`|SpawnActorFromClass` "/Game/Zombie/Blueprints/BP_Zombie.BP_Zombie_C" (`KismetMathLibrary.MakeTransform` (`NavigationSystemV1.K2_GetRandomReachablePointInRadius` (`SceneComponent.K2_GetComponentLocation` (`self.DefaultSceneRoot`)) 800.0 null null)) "AdjustIfPossibleButAlwaysSpawn" "OverrideRootScale" null null))
                (`/Engine/EditorBlueprintResources/StandardMacros.IsValid` _returnvalue
                  (:`Is Valid`
                    (`self.OnZombieSpawned` _returnvalue))
                  (:`Is Not Valid`
                    (`KismetSystemLibrary.PrintString` "not valid")))
                (else
                  (set `self.IsAllZombiesMaleWalkingDead` true))))
            (:`then_1`
              ;[1 1 1] Fait spawner les zombies male running
              (if (> (`self.waveNbr`) 3)
                (bind _returnvalue_2 (`|SpawnActorFromClass` "/Game/Zombie/Blueprints/ZombieMaleRunning/BP_ZombieMaleRunning_2.BP_ZombieMaleRunning_2_C" (`KismetMathLibrary.MakeTransform` (`NavigationSystemV1.K2_GetRandomReachablePointInRadius` (`SceneComponent.K2_GetComponentLocation` (`self.DefaultSceneRoot`)) 800.0 null null)) "AdjustIfPossibleButDontSpawnIfColliding" "OverrideRootScale" null null))
                (`/Engine/EditorBlueprintResources/StandardMacros.IsValid` _returnvalue_2
                  (:`Is Valid`
                    (`self.OnZombieMaleRunningSpawned` _returnvalue_2)))
                (else
                  (set `self.IsAllZombiesMaleRunningDead` true))))
            (:`then_2`
              ;[1 1 1] Fait spawner les zombies female walking
              (if (> (`self.waveNbr`) 1)
                (bind _returnvalue_3 (`|SpawnActorFromClass` "/Game/Zombie/Blueprints/ZombieFemalleWalking/BP_ZombieFemaleWalking.BP_ZombieFemaleWalking_C" (`KismetMathLibrary.MakeTransform` (`NavigationSystemV1.K2_GetRandomReachablePointInRadius` (`SceneComponent.K2_GetComponentLocation` (`self.DefaultSceneRoot`)) 800.0 null null)) "AdjustIfPossibleButDontSpawnIfColliding" "OverrideRootScale" null null))
                (`/Engine/EditorBlueprintResources/StandardMacros.IsValid` _returnvalue_3
                  (:`Is Valid`
                    (`self.OnZombieFemaleWalkingSpawned` _returnvalue_3)))
                (else
                  (set `self.IsAllZombiesFemaleWalkingDead` true))))
            (:`then_3`
              ;[1 1 1] Fait spawner les zombies female running
              (if (> (`self.waveNbr`) 3)
                (bind _returnvalue_4 (`|SpawnActorFromClass` "/Game/Zombie/Blueprints/ZombieFemalleRunning/BP_ZombieFemaleRunning.BP_ZombieFemaleRunning_C" (`KismetMathLibrary.MakeTransform` (`NavigationSystemV1.K2_GetRandomReachablePointInRadius` (`SceneComponent.K2_GetComponentLocation` (`self.DefaultSceneRoot`)) 800.0 null null)) "AdjustIfPossibleButDontSpawnIfColliding" "OverrideRootScale" null null))
                (`/Engine/EditorBlueprintResources/StandardMacros.IsValid` _returnvalue_4
                  (:`Is Valid`
                    (`self.OnZombieFemaleRunningSpawned` _returnvalue_4)))
                (else
                  (set `self.IsAllZombiesFemaleRunningDead` true))))))
        (:`then_1`
          (`KismetSystemLibrary.Delay` 1.0)
          (goto _label_2 :!via `Next Step In`))
        (:`then_2`
          (`KismetSystemLibrary.PrintString` "loop"))))))

(event `self.ReceiveTick`
  (params (DeltaSeconds :type "Float (single-precision)"))
  ;[1 1 1] si nbr zombies == 0, alors déclancher nouvelle vague
  (if (and (`self.IsAllZombiesMaleWalkingDead`) (`self.IsAllZombiesMaleRunningDead`) (`self.IsAllZombiesFemaleWalkingDead`) (`self.IsAllZombiesFemaleRunningDead`))
    (`KismetSystemLibrary.Delay` 1.0)
    (bind _foundwidgets (`WidgetBlueprintLibrary.GetAllWidgetsOfClass` "/Game/UI/WaveNumber2.WaveNumber2_C"))
    (`Widget.RemoveFromParent` _foundwidgets)
    (goto _label)))

(fn `createWidgets`
  (bind _wavenbr (`self.waveNbr`))
  (`|ExecutionSequence`
    (:`then_0`
      (set `self.IsAllZombiesMaleWalkingDead` false)
      (bind _returnvalue (`|CreateWidget` "/Game/UI/WaveNumber.WaveNumber_C"))
      (bind _returnvalue_2 (`|CreateWidget` "/Game/UI/WaveNumber2.WaveNumber2_C"))
      (set `/Game/UI/WaveNumber.waveNbrUi` _wavenbr _returnvalue)
      (set `/Game/UI/WaveNumber2.newWaveNumber` _wavenbr _returnvalue_2)
      (`UserWidget.AddToViewport` _returnvalue 0)
      (`UserWidget.AddToViewport` _returnvalue_2 0))
    (:`then_1`
      (set `self.IsAllZombiesMaleRunningDead` false))
    (:`then_2`
      (set `self.IsAllZombiesFemaleWalkingDead` false))
    (:`then_3`
      (set `self.IsAllZombiesFemaleRunningDead` false))))

(fn `Fun Spawn Zombies`
  ;[1 1 1] Initialisation & augmente num vague
  (set `self.waveNbr` (+ (`self.waveNbr`) 1))
  (for _ (range 1 (+ (* (`self.HordMin`) (`self.waveNbr`)) 1))
    (`|ExecutionSequence`
      (:`then_0`
        ;[1 1 1] Fait spawner les zombies male walking
        (if (> (`self.waveNbr`) 1)
          (bind _returnvalue (`|SpawnActorFromClass` "/Game/Zombie/Blueprints/BP_Zombie.BP_Zombie_C" (`KismetMathLibrary.MakeTransform` (`NavigationSystemV1.K2_GetRandomReachablePointInRadius` (`SceneComponent.K2_GetComponentLocation` (`self.DefaultSceneRoot`)) 800.0 null null)) "AdjustIfPossibleButDontSpawnIfColliding" "OverrideRootScale" null null))
          (`/Engine/EditorBlueprintResources/StandardMacros.IsValid` _returnvalue
            (:`Is Valid`
              (`self.OnZombieSpawned` _returnvalue)))
          (else
            (set `self.IsAllZombiesMaleWalkingDead` true))))
      (:`then_1`
        ;[1 1 1] Fait spawner les zombies male running
        (if (> (`self.waveNbr`) 3)
          (bind _returnvalue_2 (`|SpawnActorFromClass` "/Game/Zombie/Blueprints/ZombieMaleRunning/BP_ZombieMaleRunning_2.BP_ZombieMaleRunning_2_C" (`KismetMathLibrary.MakeTransform` (`NavigationSystemV1.K2_GetRandomReachablePointInRadius` (`SceneComponent.K2_GetComponentLocation` (`self.DefaultSceneRoot`)) 800.0 null null)) "AdjustIfPossibleButDontSpawnIfColliding" "OverrideRootScale" null null))
          (`/Engine/EditorBlueprintResources/StandardMacros.IsValid` _returnvalue_2
            (:`Is Valid`
              (`self.OnZombieMaleRunningSpawned` _returnvalue_2)))
          (else
            (set `self.IsAllZombiesMaleRunningDead` true))))
      (:`then_2`
        ;[1 1 1] Fait spawner les zombies female walking
        (if (> (`self.waveNbr`) 1)
          (bind _returnvalue_3 (`|SpawnActorFromClass` "/Game/Zombie/Blueprints/ZombieFemalleWalking/BP_ZombieFemaleWalking.BP_ZombieFemaleWalking_C" (`KismetMathLibrary.MakeTransform` (`NavigationSystemV1.K2_GetRandomReachablePointInRadius` (`SceneComponent.K2_GetComponentLocation` (`self.DefaultSceneRoot`)) 800.0 null null)) "AdjustIfPossibleButDontSpawnIfColliding" "OverrideRootScale" null null))
          (`/Engine/EditorBlueprintResources/StandardMacros.IsValid` _returnvalue_3
            (:`Is Valid`
              (`self.OnZombieFemaleWalkingSpawned` _returnvalue_3)))
          (else
            (set `self.IsAllZombiesFemaleWalkingDead` true))))
      (:`then_3`
        ;[1 1 1] Fait spawner les zombies female running
        (if (> (`self.waveNbr`) 3)
          (bind _returnvalue_4 (`|SpawnActorFromClass` "/Game/Zombie/Blueprints/ZombieFemalleRunning/BP_ZombieFemaleRunning.BP_ZombieFemaleRunning_C" (`KismetMathLibrary.MakeTransform` (`NavigationSystemV1.K2_GetRandomReachablePointInRadius` (`SceneComponent.K2_GetComponentLocation` (`self.DefaultSceneRoot`)) 800.0 null null)) "AdjustIfPossibleButDontSpawnIfColliding" "OverrideRootScale" null null))
          (`/Engine/EditorBlueprintResources/StandardMacros.IsValid` _returnvalue_4
            (:`Is Valid`
              (`self.OnZombieFemaleRunningSpawned` _returnvalue_4)))
          (else
            (set `self.IsAllZombiesFemaleRunningDead` true)))))))

(fn `OnZombieFemaleRunningKilled`
  (params (`Zombie female running` :type "/Game/Zombie/Blueprints/ZombieFemalleRunning/BP_ZombieFemaleRunning Object Reference"))
  (bind _zombiesfemalerunning (`self.ZombiesFemaleRunning`))
  (`KismetArrayLibrary.Array_RemoveItem` _zombiesfemalerunning `Zombie female running`)
  (if (<= (`KismetArrayLibrary.Array_Length` _zombiesfemalerunning) 0)
    (set `self.IsAllZombiesFemaleRunningDead` true)))

(fn `OnZombieFemaleRunningSpawned`
  (params (ZombieFemaleRunning :type "/Game/Zombie/Blueprints/ZombieFemalleRunning/BP_ZombieFemaleRunning Object Reference"))
  (`KismetArrayLibrary.Array_Add` (`self.ZombiesFemaleRunning`) ZombieFemaleRunning)
  (add `/Game/Zombie/Blueprints/ZombieFemalleRunning/BP_ZombieFemaleRunning.OnZombieFemaleRunningKilled` ZombieFemaleRunning (`|CreateDelegate` :!event `OnZombieFemaleRunningKilled`)))

(fn `OnZombieFemaleWalkingKilled`
  (params (`Zombie female walking` :type "/Game/Zombie/Blueprints/ZombieFemalleWalking/BP_ZombieFemaleWalking Object Reference"))
  (bind _zombiesfemalewalking (`self.ZombiesFemaleWalking`))
  (`KismetArrayLibrary.Array_RemoveItem` _zombiesfemalewalking `Zombie female walking`)
  (if (<= (`KismetArrayLibrary.Array_Length` _zombiesfemalewalking) 0)
    (set `self.IsAllZombiesFemaleWalkingDead` true)))

(fn `OnZombieFemaleWalkingSpawned`
  (params (`Zombie female walking` :type "/Game/Zombie/Blueprints/ZombieFemalleWalking/BP_ZombieFemaleWalking Object Reference"))
  (`KismetArrayLibrary.Array_Add` (`self.ZombiesFemaleWalking`) `Zombie female walking`)
  (add `/Game/Zombie/Blueprints/ZombieFemalleWalking/BP_ZombieFemaleWalking.OnZombieFemaleKilled` `Zombie female walking` (`|CreateDelegate` :!event `OnZombieFemaleWalkingKilled`)))

(fn `OnZombieKilled`
  (params (Zombie :type "/Game/Zombie/Blueprints/BP_Zombie Object Reference"))
  (bind _zombies (`self.Zombies`))
  ;[1 1 1] 4/ Quand un zombie est tué, le retire de l'array
  (`KismetArrayLibrary.Array_RemoveItem` _zombies Zombie)
  (if (<= (`KismetArrayLibrary.Array_Length` _zombies) 0)
    (set `self.IsAllZombiesMaleWalkingDead` true)))

(fn `OnZombieMaleRunningKilled`
  (params (BPZombieMaleRunning :type "/Game/Zombie/Blueprints/ZombieMaleRunning/BP_ZombieMaleRunning_2 Object Reference"))
  (bind _zombiesmalerunning (`self.ZombiesMaleRunning`))
  (`KismetArrayLibrary.Array_RemoveItem` _zombiesmalerunning BPZombieMaleRunning)
  (if (<= (`KismetArrayLibrary.Array_Length` _zombiesmalerunning) 0)
    (set `self.IsAllZombiesMaleRunningDead` true)))

(fn `OnZombieMaleRunningSpawned`
  (params (`Zombie male running` :type "/Game/Zombie/Blueprints/ZombieMaleRunning/BP_ZombieMaleRunning_2 Object Reference"))
  (`KismetArrayLibrary.Array_Add` (`self.ZombiesMaleRunning`) `Zombie male running`)
  (add `/Game/Zombie/Blueprints/ZombieMaleRunning/BP_ZombieMaleRunning_2.OnKilledZombieMaleRunning` `Zombie male running` (`|CreateDelegate` :!event `OnZombieMaleRunningKilled`)))

(fn `OnZombieSpawned`
  (params (Zombie :type "/Game/Zombie/Blueprints/BP_Zombie Object Reference"))
  ;[1 1 1] 3/ Une fois les zombie spawn, on les ajoutes à l'array Zombies
  (`KismetArrayLibrary.Array_Add` (`self.Zombies`) Zombie)
  (add `/Game/Zombie/Blueprints/BP_Zombie.OnKilled` Zombie (`|CreateDelegate` :!event `OnZombieKilled`)))

(fn `SpawnZombie`
  ;[1 1 1] Fait spawner les zombies male walking
  (if (> (`self.waveNbr`) 1)
    (bind _returnvalue (`|SpawnActorFromClass` "/Game/Zombie/Blueprints/BP_Zombie.BP_Zombie_C" (`KismetMathLibrary.MakeTransform` (`NavigationSystemV1.K2_GetRandomReachablePointInRadius` (`SceneComponent.K2_GetComponentLocation` (`self.DefaultSceneRoot`)) 800.0 null null)) "AdjustIfPossibleButDontSpawnIfColliding" "OverrideRootScale" null null))
    (`/Engine/EditorBlueprintResources/StandardMacros.IsValid` _returnvalue
      (:`Is Valid`
        (`self.OnZombieSpawned` _returnvalue)))
    (else
      (set `self.IsAllZombiesMaleWalkingDead` true))))

(fn `UserConstructionScript`)