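; Director actor that runs endless zombie waves, spawning them at random reachable points around itself.
; Each wave's random count scales with the wave number, capped by MaxZombies.
; Spawned zombies are tracked through kill events; once all die, Tick starts the next wave after a delay and prints the remaining count.
; Trigger-based horde spawning via BP_HorderSpawner requests remains, but its setup is disconnected and never runs.
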(event `self.ReceiveBeginPlay`
  ;[1 1 1] Début du jeu - Spawn par vague
  (set `self.waveNbr` 0)
  (`self.Fun Spawn Zombies`))

(event `self.ReceiveTick`
  (params (DeltaSeconds :type "Float (single-precision)"))
  ;[1 1 1] Affiche le nombre de zombie restant & si == 0 alors déclancher nouvelle vague
  (`|ExecutionSequence`
    (:`then_0`
      (if (`self.IsAllZombiesDead`)
        (`KismetSystemLibrary.Delay` 5.0)
        (`self.Fun Spawn Zombies`)))
    (:`then_1`
      (`KismetSystemLibrary.PrintString` (`KismetStringLibrary.Concat_StrStr` "Zombies restant :" (`KismetStringLibrary.Conv_IntToString` (`KismetArrayLibrary.Array_Length` (`self.Zombies`)))) true true (struct :`G` 0.66 :`B` 1.0 :`A` 1.0) 0.0))))

(fn `Fun Spawn Zombies`
  (bind _wavenbr (`self.waveNbr`))
  ;[1 1 1] Initialisation
  (set `self.IsAllZombiesDead` false)
  (bind _output_get (set `self.waveNbr` (+ (`self.waveNbr`) 1)))
  (`KismetSystemLibrary.PrintString` (`KismetStringLibrary.Concat_StrStr` "Wave number " (`KismetStringLibrary.Conv_IntToString` _output_get)) true true (struct :`G` 0.177542 :`B` 1.0 :`A` 1.0) 100.0)
  (for _ (range 1 (+ (`KismetMathLibrary.Min` (`KismetMathLibrary.RandomIntegerInRange` (* (`self.HordMin`) _wavenbr) (* _wavenbr (`self.HordMax`))) (- (`self.MaxZombies`) (`KismetArrayLibrary.Array_Length` (`self.Zombies`)))) 1))
    (bind _returnvalue (`|SpawnActorFromClass` "/Game/Zombie/Blueprints/BP_Zombie.BP_Zombie_C" (`KismetMathLibrary.MakeTransform` (+ (`NavigationSystemV1.K2_GetRandomReachablePointInRadius` (`SceneComponent.K2_GetComponentLocation` (`self.DefaultSceneRoot`)) 200.0 null null) (0.0 0.0 88.0))) "AdjustIfPossibleButDontSpawnIfColliding" "OverrideRootScale" null (`self.ZombieHealth`) null))
    (`/Engine/EditorBlueprintResources/StandardMacros.IsValid` _returnvalue
      (:`Is Valid`
        (`self.OnZombieSpawned` _returnvalue)))))

(fn `OnHordeSpawnerSpawned`
  (params (HorderSpawner :type "/Game/Director/BP_HorderSpawner Object Reference"))
  ;[1 1 1] 1/ Une fois la trigger box activé (BP_HorderSpawner), cette fonction est lancé
  (`KismetArrayLibrary.Array_Add` (`self.HorderSpawners`) HorderSpawner)
  (add `/Game/Director/BP_HorderSpawner.RequestSpawn` HorderSpawner (`|CreateDelegate` :!event `OnZombieSpawnRequested`)))

(fn `OnZombieKilled`
  (params (Zombie :type "/Game/Zombie/Blueprints/BP_Zombie Object Reference"))
  (bind _zombies (`self.Zombies`))
  ;[1 1 1] 4/ Quand un zombie est tué, le retire de l'array
  (`KismetArrayLibrary.Array_RemoveItem` _zombies Zombie)
  (if (<= (`KismetArrayLibrary.Array_Length` _zombies) 0)
    (`KismetSystemLibrary.PrintString` "Tout les zombies sont morts")
    (set `self.IsAllZombiesDead` true)))

(fn `OnZombieSpawned`
  (params (Zombie :type "/Game/Zombie/Blueprints/BP_Zombie Object Reference"))
  ;[1 1 1] 3/ Une fois les zombie spawn, on les ajoutes à l'array Zombies
  (`KismetArrayLibrary.Array_Add` (`self.Zombies`) Zombie)
  (add `/Game/Zombie/Blueprints/BP_Zombie.OnKilled` Zombie (`|CreateDelegate` :!event `OnZombieKilled`)))

(fn `OnZombieSpawnRequested`
  (params (Count :type Integer) (Location :type "Vector Structure"))
  ;[1 1 1] 2/ Déclanche la boucle pour faire spawn les zombies
  (for _ (range 1 (+ (`KismetMathLibrary.Min` Count (- (`self.MaxZombies`) (`KismetArrayLibrary.Array_Length` (`self.Zombies`)))) 1))
    (bind _returnvalue (`|SpawnActorFromClass` "/Game/Zombie/Blueprints/BP_Zombie.BP_Zombie_C" (`KismetMathLibrary.MakeTransform` (+ (`NavigationSystemV1.K2_GetRandomReachablePointInRadius` (`local.Location`) 200.0 null null) (0.0 0.0 88.0))) "AdjustIfPossibleButDontSpawnIfColliding" "OverrideRootScale" null 1 null))
    (`/Engine/EditorBlueprintResources/StandardMacros.IsValid` _returnvalue
      (:`Is Valid`
        (`self.OnZombieSpawned` _returnvalue)))))

(fn `UserConstructionScript`)