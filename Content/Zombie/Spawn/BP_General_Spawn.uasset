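; BP_General_Spawn is an early test Blueprint in the zombie spawn folder that checks a reference to a male running zombie spawner.
; On BeginPlay it casts SpawnerZombieMaleRunning to BP_SpawnerZombieMaleRunning and prints whether the cast succeeded.
; A disconnected debug print of the spawner's TestVar never runs, and the graph contains no spawning logic.
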(event `self.ReceiveBeginPlay`
  ;[1 1 1] Cast failed
  (cast `/Game/Zombie/Blueprints/ZombieMaleRunning/BP_SpawnerZombieMaleRunning` (`self.Spawner Zombie Male Running`)
    (:`then`
      (`KismetSystemLibrary.PrintString` "Cast success"))
    (:`CastFailed`
      (`KismetSystemLibrary.PrintString` "Cast failed" true true (struct :`R` 1.0 :`G` 0.14577 :`A` 1.0)))))

(fn `UserConstructionScript`)