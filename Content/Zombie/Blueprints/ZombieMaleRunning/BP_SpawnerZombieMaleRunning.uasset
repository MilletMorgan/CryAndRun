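; Wave spawner for running male zombies, starting the first wave on BeginPlay.
; Each wave spawns a random count scaled by wave number and capped by MaxZombies, at random reachable navmesh points around the spawner.
; Spawned zombies are tracked in an array via killed events; when it empties, a flag polled on Tick starts the next wave after a delay.
; A separate function spawns a requested count at a given location.
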(event `self.ReceiveBeginPlay`
  ;[1 1 1] Début du jeu - Spawn par vague
  (`|ExecutionSequence`
    (:`then_0`
      (set `self.waveNbr` 0)
      (`self.Func Spawn ZombieRunningMale`))))

(event `self.ReceiveTick`
  (params (DeltaSeconds :type "Float (single-precision)"))
  ;[1 1 1] Affiche le nombre de zombie restant & si == 0 alors déclancher nouvelle vague
  (`|ExecutionSequence`
    (:`then_0`
      (if (`self.IsAllZombiesDead`)
        (`KismetSystemLibrary.Delay` 5.0)
        (`self.Func Spawn ZombieRunningMale`)))))

(fn `Func Spawn ZombieRunningMale`
  (bind _wavenbr (`self.waveNbr`))
  ;[1 1 1] Initialisation
  (set `self.IsAllZombiesDead` false)
  (set `self.waveNbr` (+ (`self.waveNbr`) 1))
  (for _ (range 1 (+ (`KismetMathLibrary.Min` (`KismetMathLibrary.RandomIntegerInRange` (* (`self.HordMin`) _wavenbr) (* _wavenbr (`self.HordMax`))) (- (`self.MaxZombies`) (`KismetArrayLibrary.Array_Length` (`self.ZombiesMaleRunning`)))) 1))
    (bind _returnvalue (`|SpawnActorFromClass` "/Game/Zombie/Blueprints/ZombieMaleRunning/BP_ZombieMaleRunning.BP_ZombieMaleRunning_C" (`KismetMathLibrary.MakeTransform` (+ (`NavigationSystemV1.K2_GetRandomReachablePointInRadius` (`SceneComponent.K2_GetComponentLocation` (`self.DefaultSceneRoot`)) 200.0 null null) (0.0 0.0 88.0))) "AdjustIfPossibleButDontSpawnIfColliding" "OverrideRootScale" null (`self.ZombieHealth`) null))
    (`/Engine/EditorBlueprintResources/StandardMacros.IsValid` _returnvalue
      (:`Is Valid`
        (`self.OnZombieMaleRunningSpawned` _returnvalue)))))

(fn `OnZombieMaleRunningKilled`
  (params (ZombieMaleRunning :type "/Game/Zombie/Blueprints/ZombieMaleRunning/BP_ZombieMaleRunning Object Reference"))
  (bind _zombiesmalerunning (`self.ZombiesMaleRunning`))
  (`KismetSystemLibrary.PrintString` "On zombie male running killed")
  (`KismetArrayLibrary.Array_RemoveItem` _zombiesmalerunning ZombieMaleRunning)
  (if (<= (`KismetArrayLibrary.Array_Length` _zombiesmalerunning) 0)
    (set `self.IsAllZombiesDead` true)
    (`KismetSystemLibrary.PrintString` "dead ?" true true (struct :`R` 1.0 :`G` 0.376997 :`A` 1.0))))

(fn `OnZombieMaleRunningSpawned`
  (params (ZombieRunningMale :type "/Game/Zombie/Blueprints/ZombieMaleRunning/BP_ZombieMaleRunning Object Reference"))
  ;[1 1 1] 3/ Une fois les zombie spawn, on les ajoutes à l'array Zombies
  (`KismetArrayLibrary.Array_Add` (`self.ZombiesMaleRunning`) ZombieRunningMale)
  (add `/Game/Zombie/Blueprints/ZombieMaleRunning/BP_ZombieMaleRunning.OnKilledZombieMaleRunning` ZombieRunningMale (`|CreateDelegate` :!event `OnZombieMaleRunningKilled`)))

(fn `OnZombieSpawnRequested`
  (params (Count :type Integer) (Location :type "Vector Structure"))
  ;[1 1 1] 2/ Déclanche la boucle pour faire spawn les zombies
  (for _ (range 1 (+ (`KismetMathLibrary.Min` Count (- (`self.MaxZombies`) (`KismetArrayLibrary.Array_Length` (`self.ZombiesMaleRunning`)))) 1))
    (bind _returnvalue (`|SpawnActorFromClass` "/Game/Zombie/Blueprints/ZombieMaleRunning/BP_ZombieMaleRunning.BP_ZombieMaleRunning_C" (`KismetMathLibrary.MakeTransform` (+ (`NavigationSystemV1.K2_GetRandomReachablePointInRadius` (`local.Location`) 200.0 null null) (0.0 0.0 88.0))) "AdjustIfPossibleButDontSpawnIfColliding" "OverrideRootScale" null 1 null))
    (`/Engine/EditorBlueprintResources/StandardMacros.IsValid` _returnvalue
      (:`Is Valid`
        (`self.OnZombieMaleRunningSpawned` _returnvalue)))))

(fn `UserConstructionScript`)