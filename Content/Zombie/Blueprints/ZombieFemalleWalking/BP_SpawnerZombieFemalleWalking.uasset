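; Wave spawner for walking female zombies that starts on BeginPlay and spawns around itself at random reachable points.
; Each wave scales its random count by wave number, capped by MaxZombies.
; Registered horde spawners can request extra spawns at their own location under the same cap.
; Kill events shrink the tracked array; when it empties, Tick starts the next wave after a short Delay.
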(event `self.ReceiveBeginPlay`
  ;[1 1 1] Début du jeu - Spawn par vague
  (set `self.waveNbr` 0)
  (`self.Func Spawn ZombieWalkingFemalle`))

(event `self.ReceiveTick`
  (params (DeltaSeconds :type "Float (single-precision)"))
  ;[1 1 1] Affiche le nombre de zombie restant & si == 0 alors déclancher nouvelle vague
  (`|ExecutionSequence`
    (:`then_0`
      (if (`self.IsAllZombiesDead`)
        (`KismetSystemLibrary.Delay` 5.0)
        (`self.Func Spawn ZombieWalkingFemalle`)))))

(fn `Func Spawn ZombieWalkingFemalle`
  (bind _wavenbr (`self.waveNbr`))
  ;[1 1 1] Initialisation
  (set `self.IsAllZombiesDead` false)
  (set `self.waveNbr` (+ (`self.waveNbr`) 1))
  (for _ (range 1 (+ (`KismetMathLibrary.Min` (`KismetMathLibrary.RandomIntegerInRange` (* (`self.HordMin`) _wavenbr) (* _wavenbr (`self.HordMax`))) (- (`self.MaxZombies`) (`KismetArrayLibrary.Array_Length` (`self.ZombiesFemalleWalking`)))) 1))
    (bind _returnvalue (`|SpawnActorFromClass` "/Game/Zombie/Blueprints/ZombieFemalleWalking/BP_ZombieFemalleWalking.BP_ZombieFemalleWalking_C" (`KismetMathLibrary.MakeTransform` (+ (`NavigationSystemV1.K2_GetRandomReachablePointInRadius` (`SceneComponent.K2_GetComponentLocation` (`self.DefaultSceneRoot`)) 200.0 null null) (0.0 0.0 88.0))) "AdjustIfPossibleButDontSpawnIfColliding" "OverrideRootScale" null (`self.ZombieHealth`) null))
    (`/Engine/EditorBlueprintResources/StandardMacros.IsValid` _returnvalue
      (:`Is Valid`
        (`self.OnZombieFemalleWalkingSpawned` _returnvalue)))))

(fn `OnHordeSpawnerSpawned`
  (params (HorderSpawner :type "/Game/Director/BP_HorderSpawner Object Reference"))
  ;[1 1 1] 1/ Une fois la trigger box activé (BP_HorderSpawner), cette fonction est lancé
  (`KismetArrayLibrary.Array_Add` (`self.HorderSpawners`) HorderSpawner)
  (add `/Game/Director/BP_HorderSpawner.RequestSpawn` HorderSpawner (`|CreateDelegate` :!event `OnZombieSpawnRequested`)))

(fn `OnZombieFemalleWalkingKilled`
  (params (ZombieMaleWalking :type "/Game/Zombie/Blueprints/ZombieFemalleWalking/BP_ZombieFemalleWalking Object Reference"))
  (bind _zombiesfemallewalking (`self.ZombiesFemalleWalking`))
  (`KismetArrayLibrary.Array_RemoveItem` _zombiesfemallewalking ZombieMaleWalking)
  (if (<= (`KismetArrayLibrary.Array_Length` _zombiesfemallewalking) 0)
    (set `self.IsAllZombiesDead` true)))

(fn `OnZombieFemalleWalkingSpawned`
  (params (ZombieWalkingFemalle :type "/Game/Zombie/Blueprints/ZombieFemalleWalking/BP_ZombieFemalleWalking Object Reference"))
  ;[1 1 1] 3/ Une fois les zombie spawn, on les ajoutes à l'array Zombies
  (`KismetArrayLibrary.Array_Add` (`self.ZombiesFemalleWalking`) ZombieWalkingFemalle)
  (add `/Game/Zombie/Blueprints/ZombieFemalleWalking/BP_ZombieFemalleWalking.OnKilledZombieFemmaleWalking` ZombieWalkingFemalle (`|CreateDelegate` :!event `OnZombieFemalleWalkingSpawned`)))

(fn `OnZombieSpawnRequested`
  (params (Count :type Integer) (Location :type "Vector Structure"))
  ;[1 1 1] 2/ Déclanche la boucle pour faire spawn les zombies
  (for _ (range 1 (+ (`KismetMathLibrary.Min` Count (- (`self.MaxZombies`) (`KismetArrayLibrary.Array_Length` (`self.ZombiesFemalleWalking`)))) 1))
    (bind _returnvalue (`|SpawnActorFromClass` "/Game/Zombie/Blueprints/ZombieFemalleWalking/BP_ZombieFemalleWalking.BP_ZombieFemalleWalking_C" (`KismetMathLibrary.MakeTransform` (+ (`NavigationSystemV1.K2_GetRandomReachablePointInRadius` (`local.Location`) 200.0 null null) (0.0 0.0 88.0))) "AdjustIfPossibleButDontSpawnIfColliding" "OverrideRootScale" null 1 null))
    (`/Engine/EditorBlueprintResources/StandardMacros.IsValid` _returnvalue
      (:`Is Valid`
        (`self.OnZombieFemalleWalkingSpawned` _returnvalue)))))

(fn `UserConstructionScript`)