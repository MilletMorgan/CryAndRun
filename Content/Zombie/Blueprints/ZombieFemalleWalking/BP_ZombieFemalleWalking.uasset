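; Female walking zombie enemy that stands up on spawn, chases the player and attacks in melee.
; An AI MoveTo loop triggers timed attacks, with damage applied by mesh hits during a brief Attack window and a level load on player death.
; TakeDamage triggers KillOneZombie, which pays money, plays dying and destroys the actor, then notifies via a dispatcher.
; MarcheRandom wanders once the player is flagged dead; duplicate move/hit events and unwired logic remain.
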(event `KillOneZombie`
  ;[1 1 1] Quand un zombie est tué + donne de l'argent
  (set `self.Dead` true)
  (bind _asfirst_person_character (cast `/Game/FirstPersonBP/Blueprints/FirstPersonCharacter` (`GameplayStatics.GetPlayerPawn` 0)))
  (set `/Game/FirstPersonBP/Blueprints/FirstPersonCharacter.Money` (+ (`/Game/FirstPersonBP/Blueprints/FirstPersonCharacter.Money` _asfirst_person_character) 40) _asfirst_person_character)
  (`SkeletalMeshComponent.ResetAnimInstanceDynamics` (`self.Mesh`) "None")
  (`MovementComponent.StopMovementImmediately` (`self.CharacterMovement`))
  (`SkeletalMeshComponent.PlayAnimation` (`self.Mesh`) "/Game/Zombie/Resources/Walking/female/zombie_meuf1_Zombie_Dying.zombie_meuf1_Zombie_Dying" false)
  (`KismetSystemLibrary.Delay` 10.0)
  (`PrimitiveComponent.SetCollisionEnabled` (`self.Mesh`) "NoCollision")
  (`PrimitiveComponent.SetCollisionEnabled` (`self.CapsuleComponent`) "NoCollision")
  (`KismetSystemLibrary.Delay` 7.0)
  (`self.K2_DestroyActor`))

(event `self.ReceiveBeginPlay`
  (bind _dead (`self.Dead`))
  (bind _mesh (`self.Mesh`))
  ;[1 1 1] Quand le zombie spawn
  (`PrimitiveComponent.SetCollisionEnabled` (`self.CapsuleComponent`) "NoCollision")
  (`PrimitiveComponent.SetCollisionEnabled` _mesh "NoCollision")
  (`SkeletalMeshComponent.PlayAnimation` _mesh "/Game/Zombie/Resources/Walking/female/zombie_meuf1_Stand_Up_Anim.zombie_meuf1_Stand_Up_Anim" false)
  (if (not _dead)
    (`KismetSystemLibrary.Delay` 0.37)
    (`PrimitiveComponent.SetCollisionEnabled` (`self.CapsuleComponent`) "QueryAndPhysics")
    (`PrimitiveComponent.SetCollisionEnabled` (`self.Mesh`) "QueryAndPhysics")
    (if (not _dead)
      (`KismetSystemLibrary.Delay` 0.3)
      (if (not _dead)
        (`KismetSystemLibrary.Delay` 0.3)
        (if (not _dead)
          (`KismetSystemLibrary.Delay` 0.3)
          (if (not _dead)
            (`KismetSystemLibrary.Delay` 0.3)
            (`SkeletalMeshComponent.SetAnimInstanceClass` (`self.Mesh`) "/Game/Zombie/Resources/Walking/female/Anim_Zombie_Femelle_Walking.Anim_Zombie_Femelle_Walking_C")
            (`self.MoveToPlayer`)))))))

(event `AttackPlayerEvent`
  ;[1 1 1] Attaque le joueur
  (set `self.AttackPlayer_v` true)
  (`MovementComponent.StopMovementImmediately` (`self.CharacterMovement`))
  (`KismetSystemLibrary.Delay` 1.2)
  (set `self.Attack` true)
  (`KismetSystemLibrary.Delay` 0.2)
  (set `self.Attack` false)
  (`MovementComponent.StopMovementImmediately` (`self.CharacterMovement`))
  (`KismetSystemLibrary.Delay` 1.0)
  (set `self.AttackPlayer_v` false)
  (`self.MoveToPlayer`))

(event `MoveToPlayer`
  ;[1 1 1] Attaque le joueur
  (if (`/Game/FirstPersonBP/Blueprints/FirstPersonCharacter.PlayerDead` (stale `self.Mesh.OnComponentHit` _asfirst_person_character))
    (`self.MarcheRandom`)
    (elif (not (`self.Dead`))
      (`|AIMoveTo` self (0.0 0.0 0.0) (`GameplayStatics.GetPlayerPawn` 0)
        (:`OnSuccess`
          (`self.AttackPlayerEvent`))
        (:`OnFail`
          (`self.MoveToPlayer`))))))

(event `self.Mesh.OnComponentHit`
  (params (HitComponent :type "PrimitiveComponent Object Reference") (OtherActor :type "Actor Object Reference") (OtherComp :type "PrimitiveComponent Object Reference") (NormalImpulse :type "Vector Structure") (Hit :type "HitResult Structure (by ref)"))
  ;[1 1 1] Attaque le joueur
  (bind _asfirst_person_character (cast `/Game/FirstPersonBP/Blueprints/FirstPersonCharacter` OtherActor))
  (if (`self.Attack`)
    (set `/Game/FirstPersonBP/Blueprints/FirstPersonCharacter.CurHealth` (- (`/Game/FirstPersonBP/Blueprints/FirstPersonCharacter.CurHealth` _asfirst_person_character) 40) _asfirst_person_character)
    (set `self.Attack` false)
    (`KismetSystemLibrary.Delay` 2.2)
    (if (<= (`/Game/FirstPersonBP/Blueprints/FirstPersonCharacter.CurHealth` _asfirst_person_character) 0)
      (`KismetSystemLibrary.PrintString` "t'es mort")
      (`KismetSystemLibrary.Delay` 3.0)
      (`GameplayStatics.OpenLevel` "Mort")
      (else
        (`KismetSystemLibrary.PrintString` (`KismetStringLibrary.Conv_IntToString` (`/Game/FirstPersonBP/Blueprints/FirstPersonCharacter.CurHealth` _asfirst_person_character)))))))

(event `MarcheRandom`
  ;[1 1 1] Marche aléatoire
  (`KismetSystemLibrary.PrintString` "random")
  (`|AIMoveTo` null (`NavigationSystemV1.K2_GetRandomLocationInNavigableRadius` (`self.K2_GetActorLocation`) 6000.0 null null) null))

(event `MoveToPlayer2`
  ;[1 1 1] Se déplace vers le joueur
  (if (`/Game/FirstPersonBP/Blueprints/FirstPersonCharacter.PlayerDead` (stale `CustomEvent_1` _asfirst_person_character))
    (`self.MarcheRandom`)
    (elif (not (`self.Dead`))
      (`|AIMoveTo` self (0.0 0.0 0.0) (`GameplayStatics.GetPlayerPawn` 0) 0.5
        (:`OnSuccess`
          (`self.AttackPlayerEvent`))
        (:`OnFail`
          (`self.MoveToPlayer`))))))

(event `CustomEvent_1`
  (params (HitComponent :type "PrimitiveComponent Object Reference") (OtherActor :type "Actor Object Reference") (OtherComp :type "PrimitiveComponent Object Reference") (NormalImpulse :type "Vector Structure") (Hit :type "HitResult Structure (by ref)"))
  ;[1 1 1] Se déplace vers le joueur
  (bind _asfirst_person_character (cast `/Game/FirstPersonBP/Blueprints/FirstPersonCharacter` OtherActor))
  (if (`self.Attack`)
    (set `/Game/FirstPersonBP/Blueprints/FirstPersonCharacter.CurHealth` (- (`/Game/FirstPersonBP/Blueprints/FirstPersonCharacter.CurHealth` _asfirst_person_character) 40) _asfirst_person_character)
    (set `self.Attack` false)
    (bind _curhealth (`/Game/FirstPersonBP/Blueprints/FirstPersonCharacter.CurHealth` _asfirst_person_character))
    (if (<= _curhealth 0)
      (`/Game/FirstPersonBP/Blueprints/FirstPersonCharacter.Mort` _asfirst_person_character)
      (`KismetSystemLibrary.Delay` 5.0)
      (`KismetSystemLibrary.Delay` 5.0)
      (`GameplayStatics.OpenLevel` "MainMenu")
      (else
        (`KismetSystemLibrary.PrintString` (`KismetStringLibrary.Conv_IntToString` _curhealth))))))

(fn `AttackPlayer`)

(fn `TakeDamage`
  (params (DamageToTake :type Integer))
  ;[1 1 1] Comment
  (bind _output_get (set `self.Health` (- (`self.Health`) DamageToTake)))
  (if (<= _output_get 0)
    (if (not (`self.Dead`))
      (set `self.Dead` true)
      (`self.KillOneZombie`)
      (`MovementComponent.StopMovementImmediately` (`self.CharacterMovement`))
      (`self.OnKilledZombieFemmaleWalking` self))))

(fn `UserConstructionScript`)