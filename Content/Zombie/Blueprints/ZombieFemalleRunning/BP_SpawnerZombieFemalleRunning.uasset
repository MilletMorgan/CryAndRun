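; Wave spawner that releases growing hordes of running female zombies, starting at BeginPlay.
; Each wave rolls a count scaled by wave number, capped by MaxZombies, and spawns zombies at random reachable points around the spawner.
; Spawned zombies are tracked in an array with kill events bound; emptying it sets a flag that Tick polls to launch the next wave after a delay.
; A separate function spawns a requested count at a given location.
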(event `self.ReceiveBeginPlay`
  ;[1 1 1] Début du jeu - Spawn par vague
  (set `self.waveNbr` 0)
  (`self.Func Spawn ZombieRunningFemalle`))

(event `self.ReceiveTick`
  (params (DeltaSeconds :type "Float (single-precision)"))
  ;[1 1 1] Affiche le nombre de zombie restant & si == 0 alors déclancher nouvelle vague
  (`|ExecutionSequence`
    (:`then_0`
      (if (`self.IsAllZombiesDead`)
        (`KismetSystemLibrary.Delay` 5.0)
        (`self.Func Spawn ZombieRunningFemalle`)))))

(fn `Func Spawn ZombieRunningFemalle`
  (bind _wavenbr (`self.waveNbr`))
  ;[1 1 1] Initialisation
  (set `self.IsAllZombiesDead` false)
  (set `self.waveNbr` (+ (`self.waveNbr`) 1))
  (for _ (range 1 (+ (`KismetMathLibrary.Min` (`KismetMathLibrary.RandomIntegerInRange` (* (`self.HordMin`) _wavenbr) (* _wavenbr (`self.HordMax`))) (- (`self.MaxZombies`) (`KismetArrayLibrary.Array_Length` (`self.ZombiesFemalleRunning`)))) 1))
    (bind _returnvalue (`|SpawnActorFromClass` "/Game/Zombie/Blueprints/ZombieFemalleRunning/BP_ZombieFemalleRunning.BP_ZombieFemalleRunning_C" (`KismetMathLibrary.MakeTransform` (+ (`NavigationSystemV1.K2_GetRandomReachablePointInRadius` (`SceneComponent.K2_GetComponentLocation` (`self.DefaultSceneRoot`)) 200.0 null null) (0.0 0.0 88.0))) "AdjustIfPossibleButDontSpawnIfColliding" "OverrideRootScale" null (`self.ZombieHealth`) null))
    (`/Engine/EditorBlueprintResources/StandardMacros.IsValid` _returnvalue
      (:`Is Valid`
        (`self.OnZombieFemalleRunningSpawned` _returnvalue)))))

(fn `OnZombieFemalleRunningKilled`
  (params (ZombieFemaleRunning :type "/Game/Zombie/Blueprints/ZombieFemalleRunning/BP_ZombieFemalleRunning Object Reference"))
  (bind _zombiesfemallerunning (`self.ZombiesFemalleRunning`))
  (`KismetArrayLibrary.Array_RemoveItem` _zombiesfemallerunning ZombieFemaleRunning)
  (if (<= (`KismetArrayLibrary.Array_Length` _zombiesfemallerunning) 0)
    (set `self.IsAllZombiesDead` true)))

(fn `OnZombieFemalleRunningSpawned`
  (params (ZombieFemalleRunning :type "/Game/Zombie/Blueprints/ZombieFemalleRunning/BP_ZombieFemalleRunning Object Reference"))
  ;[1 1 1] 3/ Une fois les zombie spawn, on les ajoutes à l'array Zombies
  (`KismetArrayLibrary.Array_Add` (`self.ZombiesFemalleRunning`) ZombieFemalleRunning)
  (add `/Game/Zombie/Blueprints/ZombieFemalleRunning/BP_ZombieFemalleRunning.OnKilledZombieFemmaleRunning` ZombieFemalleRunning (`|CreateDelegate` :!event `OnZombieFemalleRunningKilled`)))

(fn `OnZombieSpawnRequested`
  (params (Count :type Integer) (Location :type "Vector Structure"))
  ;[1 1 1] 2/ Déclanche la boucle pour faire spawn les zombies
  (for _ (range 1 (+ (`KismetMathLibrary.Min` Count (- (`self.MaxZombies`) (`KismetArrayLibrary.Array_Length` (`self.ZombiesFemalleRunning`)))) 1))
    (bind _returnvalue (`|SpawnActorFromClass` "/Game/Zombie/Blueprints/ZombieFemalleRunning/BP_ZombieFemalleRunning.BP_ZombieFemalleRunning_C" (`KismetMathLibrary.MakeTransform` (+ (`NavigationSystemV1.K2_GetRandomReachablePointInRadius` (`local.Location`) 200.0 null null) (0.0 0.0 88.0))) "AdjustIfPossibleButDontSpawnIfColliding" "OverrideRootScale" null 1 null))
    (`/Engine/EditorBlueprintResources/StandardMacros.IsValid` _returnvalue
      (:`Is Valid`
        (`self.OnZombieFemalleRunningSpawned` _returnvalue)))))

(fn `UserConstructionScript`)