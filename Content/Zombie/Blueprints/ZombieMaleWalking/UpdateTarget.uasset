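; Behavior tree service for the walking male zombie that updates its target based on the player's proximity.
; Each tick compares squared distance to player character 0 against squared PerceptionDistance, with no line-of-sight check.
; In range, it writes the player to the AITarget blackboard key and switches AIState; otherwise it clears the target and resets the state.
; An unconnected attack-state branch with a debug print never runs.
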(event `self.ReceiveTickAI`
  (params (OwnerController :type "AIController Object Reference") (ControlledPawn :type "Pawn Object Reference") (DeltaSeconds :type "Float (single-precision)"))
  (if (< (`KismetMathLibrary.Vector_DistanceSquared` (`Actor.K2_GetActorLocation` ControlledPawn) (`Actor.K2_GetActorLocation` (`GameplayStatics.GetPlayerCharacter` 0))) (`KismetMathLibrary.Square` (`self.PerceptionDistance`)))
    (`|ExecutionSequence`
      (:`then_1`
        (`BTFunctionLibrary.SetBlackboardValueAsObject` (`self.AITarget`) (`GameplayStatics.GetPlayerCharacter` 0))
        (`BTFunctionLibrary.SetBlackboardValueAsEnum` (`self.AIState`) (enumliteral `/Game/Zombie/Blueprints/ZombieMaleWalking/ZombieAIState` "NewEnumerator1"))))
    (else
      (`BTFunctionLibrary.SetBlackboardValueAsObject` (`self.AITarget`))
      (`BTFunctionLibrary.SetBlackboardValueAsEnum` (`self.AIState`) (enumliteral `/Game/Zombie/Blueprints/ZombieMaleWalking/ZombieAIState` "NewEnumerator0")))))