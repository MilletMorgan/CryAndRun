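; Male walking zombie enemy that rises on spawn, chases the player and attacks in melee.
; After the stand-up animation it switches to its walking AnimBP and loops AIMoveTo with a timed attack.
; Mesh hits during the brief Attack window damage FirstPersonCharacter, opening the "Mort" level at zero health.
; TakeDamage handles death: dying animation, capsule collision off, kill dispatcher call and delayed destroy; randomization, ragdoll and distance-attack code is unwired.
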(event `KillOneZombie`
  ;[1 1 1] Quand un zombie est tué
  (set `self.Dead` true)
  (`SkeletalMeshComponent.ResetAnimInstanceDynamics` (`self.Mesh`) "None")
  (`MovementComponent.StopMovementImmediately` (`self.CharacterMovement`))
  (`SkeletalMeshComponent.PlayAnimation` (`self.Mesh`) "/Game/Zombie/Resources/Walking/male/zombie_mec1_Mutant_Dying.zombie_mec1_Mutant_Dying" false)
  (`KismetSystemLibrary.Delay` 10.0)
  (`self.K2_DestroyActor`))

(event `self.ReceiveBeginPlay`
  (bind _dead (`self.Dead`))
  ;[1 1 1] Quand le zombie spawn
  (`SkeletalMeshComponent.PlayAnimation` (`self.Mesh`) "/Game/Zombie/Resources/Walking/male/zombie_mec1_Zombie_Stand_Up_Anim.zombie_mec1_Zombie_Stand_Up_Anim" false)
  (if (not _dead)
    (`KismetSystemLibrary.Delay` 0.37)
    (if (not _dead)
      (`KismetSystemLibrary.Delay` 0.3)
      (if (not _dead)
        (`KismetSystemLibrary.Delay` 0.3)
        (if (not _dead)
          (`KismetSystemLibrary.Delay` 0.3)
          (if (not _dead)
            (`KismetSystemLibrary.Delay` 0.3)
            (`SkeletalMeshComponent.SetAnimInstanceClass` (`self.Mesh`) "/Game/Zombie/Resources/Walking/male/AN_Zombie_Walking_Male.AN_Zombie_Walking_Male_C")
            (`self.MoveToPlayer`)))))))

(event `MoveToPlayer`
  ;[1 1 1] Se déplace vers le joueur
  (if (not (`self.Dead`))
    (`|AIMoveTo` self (0.0 0.0 0.0) (`GameplayStatics.GetPlayerPawn` 0)
      (:`OnSuccess`
        (`self.AttackPlayerEvent`))
      (:`OnFail`
        (`self.MoveToPlayer`)))))

(event `AttackPlayerEvent`
  ;[1 1 1] Attaque le joueur
  (set `self.AttackPlayer_v` true)
  (`MovementComponent.StopMovementImmediately` (`self.CharacterMovement`))
  (`KismetSystemLibrary.Delay` 1.2)
  (set `self.Attack` true)
  (`KismetSystemLibrary.Delay` 0.2)
  (set `self.Attack` false)
  (`MovementComponent.StopMovementImmediately` (`self.CharacterMovement`))
  (`KismetSystemLibrary.Delay` 1.0)
  (set `self.AttackPlayer_v` false)
  (`self.MoveToPlayer`))

(event `self.Mesh.OnComponentHit`
  (params (HitComponent :type "PrimitiveComponent Object Reference") (OtherActor :type "Actor Object Reference") (OtherComp :type "PrimitiveComponent Object Reference") (NormalImpulse :type "Vector Structure") (Hit :type "HitResult Structure (by ref)"))
  ;[1 1 1] Attaque le joueur
  (bind _asfirst_person_character (cast `/Game/FirstPersonBP/Blueprints/FirstPersonCharacter` OtherActor))
  (if (`self.Attack`)
    (set `/Game/FirstPersonBP/Blueprints/FirstPersonCharacter.CurHealth` (- (`/Game/FirstPersonBP/Blueprints/FirstPersonCharacter.CurHealth` _asfirst_person_character) 40) _asfirst_person_character)
    (set `self.Attack` false)
    (`KismetSystemLibrary.Delay` 2.2)
    (if (<= (`/Game/FirstPersonBP/Blueprints/FirstPersonCharacter.CurHealth` _asfirst_person_character) 0)
      (`KismetSystemLibrary.PrintString` "t'es mort")
      (`KismetSystemLibrary.Delay` 3.0)
      (`GameplayStatics.OpenLevel` "Mort")
      (else
        (`KismetSystemLibrary.PrintString` (`KismetStringLibrary.Conv_IntToString` (`/Game/FirstPersonBP/Blueprints/FirstPersonCharacter.CurHealth` _asfirst_person_character)))))))

(fn `AttackPlayer`)

(fn `TakeDamage`
  (params (DamageToTake :type Integer))
  ;[1 1 1] Comment
  (bind _output_get (set `self.Health` (- (`self.Health`) DamageToTake)))
  (if (<= _output_get 0)
    (set `self.Dead` true)
    (`self.KillOneZombie`)
    (`MovementComponent.StopMovementImmediately` (`self.CharacterMovement`))
    (`PrimitiveComponent.SetCollisionProfileName` (`self.CapsuleComponent`) "NoCollision" true)
    (`self.OnKilledZombieMaleWalking` self)))

(fn `UserConstructionScript`)