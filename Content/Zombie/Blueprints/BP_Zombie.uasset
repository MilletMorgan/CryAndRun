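; Zombie enemy that rises on spawn, chases and attacks the player, and awards kills, money and score when killed.
; Bullet overlaps on body-part colliders call TakeDamage with location-based damage, gated by a brief Attackable cooldown.
; AIMoveTo loops into timed attacks whose mesh hits damage the player, triggering revive or death and menu return; it wanders once the player is dead.
; High-score save logic is present but disconnected.
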(event `KillOneZombie`
  ;[1 1 1] Set le score & l'argents et les kills
  (set `self.Dead` true)
  (bind _asfirst_person_character (cast `/Game/FirstPersonBP/Blueprints/FirstPersonCharacter` (`GameplayStatics.GetPlayerPawn` 0)))
  (`|ExecutionSequence`
    (:`then_0`
      (`SkeletalMeshComponent.ResetAnimInstanceDynamics` (`self.Mesh`) "None")
      (`MovementComponent.StopMovementImmediately` (`self.CharacterMovement`))
      (`SkeletalMeshComponent.PlayAnimation` (`self.Mesh`) "/Game/Zombie/Resources/Walking/male/zombie_mec1_Mutant_Dying.zombie_mec1_Mutant_Dying" false)
      (`KismetSystemLibrary.Delay` 3.0)
      (`PrimitiveComponent.SetCollisionEnabled` (`self.Mesh`) "NoCollision")
      (`PrimitiveComponent.SetCollisionEnabled` (`self.CapsuleComponent`) "NoCollision")
      (`KismetSystemLibrary.Delay` 7.0)
      (`self.K2_DestroyActor`))
    (:`then_1`
      (set `/Game/FirstPersonBP/Blueprints/FirstPersonCharacter.Kills` (+ (`/Game/FirstPersonBP/Blueprints/FirstPersonCharacter.Kills` _asfirst_person_character) 1) _asfirst_person_character))
    (:`then_2`
      (set `/Game/FirstPersonBP/Blueprints/FirstPersonCharacter.Money` (+ (`/Game/FirstPersonBP/Blueprints/FirstPersonCharacter.Money` _asfirst_person_character) 40) _asfirst_person_character))
    (:`then_3`
      (bind _output_get (set `/Game/FirstPersonBP/Blueprints/FirstPersonCharacter.Score` (+ (`/Game/FirstPersonBP/Blueprints/FirstPersonCharacter.Score` _asfirst_person_character) 40) _asfirst_person_character)))))

(event `self.head.OnComponentBeginOverlap`
  (params (OverlappedComponent :type "PrimitiveComponent Object Reference") (OtherActor :type "Actor Object Reference") (OtherComp :type "PrimitiveComponent Object Reference") (OtherBodyIndex :type Integer) (bFromSweep :type Boolean) (SweepResult :type "HitResult Structure (by ref)"))
  ;[1 1 1] Degats Tete
  (bind _asbullet (cast `/Game/FirstPersonBP/Bullet/Bullet` OtherActor))
  (`self.TakeDamage` 100 _asbullet)
  (`KismetSystemLibrary.Delay` 0.2)
  (set `self.attackable` true))

(event `self.ReceiveBeginPlay`
  (bind _dead (`self.Dead`))
  (bind _mesh (`self.Mesh`))
  ;[1 1 1] Quand le zombie spawn
  (`|ExecutionSequence`
    (:`then_0`
      (`PrimitiveComponent.SetCollisionEnabled` (`self.CapsuleComponent`) "NoCollision")
      (`PrimitiveComponent.SetCollisionEnabled` _mesh "NoCollision")
      (`SkeletalMeshComponent.PlayAnimation` _mesh "/Game/Zombie/Resources/Walking/male/zombie_mec1_Zombie_Stand_Up_Anim.zombie_mec1_Zombie_Stand_Up_Anim" false)
      (if (not _dead)
        (`KismetSystemLibrary.Delay` 0.37)
        (`PrimitiveComponent.SetCollisionEnabled` (`self.CapsuleComponent`) "QueryAndPhysics")
        (`PrimitiveComponent.SetCollisionEnabled` (`self.Mesh`) "QueryAndPhysics")
        (if (not _dead)
          (`KismetSystemLibrary.Delay` 0.3)
          (if (not _dead)
            (`KismetSystemLibrary.Delay` 0.3)
            (if (not _dead)
              (`KismetSystemLibrary.Delay` 0.3)
              (if (not _dead)
                (`KismetSystemLibrary.Delay` 0.3)
                (`SkeletalMeshComponent.SetAnimInstanceClass` (`self.Mesh`) "/Game/Zombie/Resources/Walking/male/AN_Zombie_Walking_Male.AN_Zombie_Walking_Male_C")
                (`self.MoveToPlayer`)))))))))

(event `self.corps.OnComponentBeginOverlap`
  (params (OverlappedComponent :type "PrimitiveComponent Object Reference") (OtherActor :type "Actor Object Reference") (OtherComp :type "PrimitiveComponent Object Reference") (OtherBodyIndex :type Integer) (bFromSweep :type Boolean) (SweepResult :type "HitResult Structure (by ref)"))
  ;[1 1 1] Degats Torse
  (cast `/Game/FirstPersonBP/Bullet/Bullet` OtherActor)
  (`self.TakeDamage` 30)
  (`KismetSystemLibrary.Delay` 0.2)
  (set `self.attackable` true))

(event `self.LeftArm.OnComponentBeginOverlap`
  (params (OverlappedComponent :type "PrimitiveComponent Object Reference") (OtherActor :type "Actor Object Reference") (OtherComp :type "PrimitiveComponent Object Reference") (OtherBodyIndex :type Integer) (bFromSweep :type Boolean) (SweepResult :type "HitResult Structure (by ref)"))
  ;[1 1 1] Degats Bras
  (cast `/Game/FirstPersonBP/Bullet/Bullet` OtherActor)
  (`self.TakeDamage` 20)
  (`KismetSystemLibrary.Delay` 0.2)
  (set `self.attackable` true))

(event `self.RightArm.OnComponentBeginOverlap`
  (params (OverlappedComponent :type "PrimitiveComponent Object Reference") (OtherActor :type "Actor Object Reference") (OtherComp :type "PrimitiveComponent Object Reference") (OtherBodyIndex :type Integer) (bFromSweep :type Boolean) (SweepResult :type "HitResult Structure (by ref)"))
  ;[1 1 1] Degats Bras
  (cast `/Game/FirstPersonBP/Bullet/Bullet` OtherActor)
  (`self.TakeDamage` 20)
  (`KismetSystemLibrary.Delay` 0.2)
  (set `self.attackable` true))

(event `MarcheRandom`
  ;[1 1 1] Marche aléatoire
  (`|AIMoveTo` null (`NavigationSystemV1.K2_GetRandomLocationInNavigableRadius` (`self.K2_GetActorLocation`) 6000.0 null null) null
    (:`OnSuccess`
      (`self.MarcheRandom`))
    (:`OnFail`
      (`self.MarcheRandom`))))

(event `MoveToPlayer`
  ;[1 1 1] Se déplace vers le joueur
  (if (`/Game/FirstPersonBP/Blueprints/FirstPersonCharacter.PlayerDead` (stale `self.Mesh.OnComponentHit` _asfirst_person_character))
    (`self.MarcheRandom`)
    (elif (not (`self.Dead`))
      (`|AIMoveTo` self (0.0 0.0 0.0) (`GameplayStatics.GetPlayerPawn` 0) 0.5
        (:`OnSuccess`
          (`self.AttackPlayerEvent`))
        (:`OnFail`
          (`self.MoveToPlayer`))))))

(event `self.RightArm1.OnComponentBeginOverlap`
  (params (OverlappedComponent :type "PrimitiveComponent Object Reference") (OtherActor :type "Actor Object Reference") (OtherComp :type "PrimitiveComponent Object Reference") (OtherBodyIndex :type Integer) (bFromSweep :type Boolean) (SweepResult :type "HitResult Structure (by ref)"))
  ;[1 1 1] Degats Bras
  (cast `/Game/FirstPersonBP/Bullet/Bullet` OtherActor)
  (`self.TakeDamage` 20)
  (`KismetSystemLibrary.Delay` 0.2)
  (set `self.attackable` true))

(event `self.LeftArm1.OnComponentBeginOverlap`
  (params (OverlappedComponent :type "PrimitiveComponent Object Reference") (OtherActor :type "Actor Object Reference") (OtherComp :type "PrimitiveComponent Object Reference") (OtherBodyIndex :type Integer) (bFromSweep :type Boolean) (SweepResult :type "HitResult Structure (by ref)"))
  ;[1 1 1] Degats Bras
  (cast `/Game/FirstPersonBP/Bullet/Bullet` OtherActor)
  (`self.TakeDamage` 20)
  (`KismetSystemLibrary.Delay` 0.2)
  (set `self.attackable` true))

(event `self.Mesh.OnComponentHit`
  (params (HitComponent :type "PrimitiveComponent Object Reference") (OtherActor :type "Actor Object Reference") (OtherComp :type "PrimitiveComponent Object Reference") (NormalImpulse :type "Vector Structure") (Hit :type "HitResult Structure (by ref)"))
  ;[1 1 1] Le Zombie se prend des dégats
  (bind _asfirst_person_character (cast `/Game/FirstPersonBP/Blueprints/FirstPersonCharacter` OtherActor))
  (if (`self.Attack`)
    (bind _curhealth (`/Game/FirstPersonBP/Blueprints/FirstPersonCharacter.CurHealth` _asfirst_person_character))
    (set `/Game/FirstPersonBP/Blueprints/FirstPersonCharacter.CurHealth` (- _curhealth 40) _asfirst_person_character)
    (set `self.Attack` false)
    (if (<= _curhealth 0)
      (if (`/Game/FirstPersonBP/Blueprints/FirstPersonCharacter.PlayerDead` _asfirst_person_character)
        _
        (elif (`/Game/FirstPersonBP/Blueprints/FirstPersonCharacter.reanimations` _asfirst_person_character)
          (`/Game/FirstPersonBP/Blueprints/FirstPersonCharacter.Reanimation` _asfirst_person_character)
          (else
            (`/Game/FirstPersonBP/Blueprints/FirstPersonCharacter.Mort` _asfirst_person_character)
            (`KismetSystemLibrary.Delay` 5.0)
            (`/Game/FirstPersonBP/Blueprints/FirstPersonCharacter.MortSuite` _asfirst_person_character)
            (`KismetSystemLibrary.Delay` 10.0)
            (`GameplayStatics.OpenLevel` "MainMenu")))))))

(event `self.LeftLeg.OnComponentBeginOverlap`
  (params (OverlappedComponent :type "PrimitiveComponent Object Reference") (OtherActor :type "Actor Object Reference") (OtherComp :type "PrimitiveComponent Object Reference") (OtherBodyIndex :type Integer) (bFromSweep :type Boolean) (SweepResult :type "HitResult Structure (by ref)"))
  ;[1 1 1] Degats Jambes
  (cast `/Game/FirstPersonBP/Bullet/Bullet` OtherActor)
  (`self.TakeDamage` 10)
  (`KismetSystemLibrary.Delay` 0.2)
  (set `self.attackable` true))

(event `self.LeftLeg1.OnComponentBeginOverlap`
  (params (OverlappedComponent :type "PrimitiveComponent Object Reference") (OtherActor :type "Actor Object Reference") (OtherComp :type "PrimitiveComponent Object Reference") (OtherBodyIndex :type Integer) (bFromSweep :type Boolean) (SweepResult :type "HitResult Structure (by ref)"))
  ;[1 1 1] Degats Jambes
  (cast `/Game/FirstPersonBP/Bullet/Bullet` OtherActor)
  (`self.TakeDamage` 10)
  (`KismetSystemLibrary.Delay` 0.2)
  (set `self.attackable` true))

(event `self.RightLeg.OnComponentBeginOverlap`
  (params (OverlappedComponent :type "PrimitiveComponent Object Reference") (OtherActor :type "Actor Object Reference") (OtherComp :type "PrimitiveComponent Object Reference") (OtherBodyIndex :type Integer) (bFromSweep :type Boolean) (SweepResult :type "HitResult Structure (by ref)"))
  ;[1 1 1] Degats Jambes
  (cast `/Game/FirstPersonBP/Bullet/Bullet` OtherActor)
  (`self.TakeDamage` 10)
  (`KismetSystemLibrary.Delay` 0.2)
  (set `self.attackable` true))

(event `AttackPlayerEvent`
  ;[1 1 1] Attaque le joueur
  (set `self.AttackPlayer_v` true)
  (`MovementComponent.StopMovementImmediately` (`self.CharacterMovement`))
  (`KismetSystemLibrary.Delay` 1.1)
  (set `self.Attack` true)
  (`KismetSystemLibrary.Delay` 0.5)
  (set `self.Attack` false)
  (`MovementComponent.StopMovementImmediately` (`self.CharacterMovement`))
  (`KismetSystemLibrary.Delay` 0.7)
  (set `self.AttackPlayer_v` false)
  (`self.MoveToPlayer`))

(event `self.RightLeg2.OnComponentBeginOverlap`
  (params (OverlappedComponent :type "PrimitiveComponent Object Reference") (OtherActor :type "Actor Object Reference") (OtherComp :type "PrimitiveComponent Object Reference") (OtherBodyIndex :type Integer) (bFromSweep :type Boolean) (SweepResult :type "HitResult Structure (by ref)"))
  ;[1 1 1] Degats Jambes
  (cast `/Game/FirstPersonBP/Bullet/Bullet` OtherActor)
  (`self.TakeDamage` 10)
  (`KismetSystemLibrary.Delay` 0.2)
  (set `self.attackable` true))

(fn `TakeDamage`
  (params (DamageToTake :type Integer) (bullet :type "/Game/FirstPersonBP/Bullet/Bullet Object Reference"))
  (if (`self.Dead`)
    _
    (elif (`self.attackable`)
      (set `self.MaxHealthZ` (- (`self.MaxHealthZ`) DamageToTake))
      (set `self.attackable` false)
      (`self.K2_DestroyActor` bullet)
      (if (<= (`self.MaxHealthZ`) 0)
        (if (not (`self.Dead`))
          (set `self.Dead` true)
          (`self.KillOneZombie`)
          (`MovementComponent.StopMovementImmediately` (`self.CharacterMovement`))
          (`self.OnKilled` self))))))

(fn `UserConstructionScript`)