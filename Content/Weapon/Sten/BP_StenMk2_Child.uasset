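; Child Blueprint of a Sten Mk2 weapon that handles the player acquiring the gun through the AcheterArme ("buy weapon") event.
; The event calls PickupRifleMessage on player 0's FirstPersonCharacter and snaps the weapon to the socketArme socket on its mesh.
; It then hides the widget, destroys the sphere component and turns off custom depth rendering on the skeletal mesh.
; Construction only runs the parent script.
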(event `AcheterArme`
  (bind _asfirst_person_character (cast `/Game/FirstPersonBP/Blueprints/FirstPersonCharacter` (`GameplayStatics.GetPlayerCharacter` 0)))
  (message `/Game/Weapon/PickUp_Weapon.PickupRifle` _asfirst_person_character)
  (`self.K2_AttachToComponent` self (`Character.Mesh` _asfirst_person_character) "socketArme" "SnapToTarget" "SnapToTarget" "SnapToTarget" true)
  (`SceneComponent.SetVisibility` (`self.Widget`) false false)
  (`ActorComponent.K2_DestroyComponent` (`self.Sphere`))
  (`PrimitiveComponent.SetRenderCustomDepth` (`self.SkeletalMesh`) false))

(fn `UserConstructionScript`
  (`parent.UserConstructionScript`))